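; Crystal interactable that fires once when the player character overlaps it, starting a level interaction; its Interact interface event is empty.
; It activates the player's rain message, calls the level interaction, plays a start sound, and sets location and level on the rhythm game mode's AudioManager.
; The crystal brightens while player input is disabled for a short delay, then input returns and the crystal turns red.
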(event Collision|EventActorBeginOverlap
  (params (OtherActor :type Actor%20Object%20Reference))
  (bind _returnvalue (Game|GetPlayerCharacter 0))
  (if (== OtherActor _returnvalue)
    (if (not (Variables|Default|GetUsed?))
      (Variables|Default|SetUsed? true)
      (Variables|Default|SetIsActive true)
      (bind _raincomponent (Class|IPlayerUtilities|IGetRain(Message) _returnvalue))
      (Components|Activation|Activate _raincomponent false)
      (Default|CallLevelInteraction)
      (Class|FMODBlueprintStatics|PlayEvent2D "/Game/FMOD/Events/SFX/StartLevel.StartLevel")
      (bind _asbp_rhythm_game_mode (Utilities|Casting|CastToBP_RhythmGameMode (Game|GetGameMode)))
      (bind _audiomanager (Default|GetAudioManager _asbp_rhythm_game_mode))
      (Default|SetGameLocation _audiomanager 2)
      (Rendering|Material|SetMaterial (Variables|Default|GetCrystal) 0 "/Game/Crystal_cave/Materials/MI_crystal_bright.MI_crystal_bright")
      ;[1 1 1] Disable player inputs
      (bind _asbp_third_person_character (Utilities|Casting|CastToBP_ThirdPersonCharacter (Game|GetPlayerCharacter 0)))
      (Default|SetPlayerInputs _asbp_third_person_character false)
      ;[1 1 1] Update level in AudioManager
      (bind _asbp_rhythm_game_mode_2 (Utilities|Casting|CastToBP_RhythmGameMode (Game|GetGameMode)))
      (bind _audiomanager_2 (Default|GetAudioManager _asbp_rhythm_game_mode_2))
      (Default|SetGameLevel _audiomanager_2 (Variables|Default|GetLevel))
      (Utilities|FlowControl|Delay 2.5)
      (Default|SetPlayerInputs _asbp_third_person_character true)
      (Rendering|Material|SetMaterial (Variables|Default|GetCrystal) 0 "/Game/Blueprints/MI_CrystalRed.MI_CrystalRed"))))

(event EventIInteractwith)

(fn ConstructionScript)