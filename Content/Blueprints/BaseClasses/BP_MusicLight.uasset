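; BP_MusicLight is a music-driven light actor that flashes a point light whenever its Play function is called.
; Play runs the parent implementation, then fires LightIntensityEvent, which sets the light color and restarts a timeline that scales intensity up to MaxLightInt.
; An unconnected leftover chain would find the first BP_KickTower and bind to its kick dispatcher, but it never runs.
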(event Custom|LightIntensityEvent
  (bind _pointlight (Variables|Default|GetPointLight))
  (Rendering|Components|Light|SetLightColor _pointlight (Math|Conversions|ToLinearColor(Color) (Variables|Default|GetLightColor)) true)
  (bind _lightintensityanim (Timeline|LightAnimation PlayFromStart)
    (:Update
      (Rendering|Components|Light|SetIntensity _pointlight (* _lightintensityanim (Variables|Default|GetMaxLightInt))))))

(event EventBeginPlay)

(event Collision|EventActorBeginOverlap
  (params (OtherActor :type Actor%20Object%20Reference)))

(event EventTick
  (params (DeltaSeconds :type Float%20%28single-precision%29)))

(fn ConstructionScript)

(fn Play
  (|CallParentFunction)
  (CallFunction|LightIntensityEvent))