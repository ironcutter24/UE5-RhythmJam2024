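; Base class for music-reactive objects in a rhythm game, giving children empty Kick, Snare, Laser, Marker and Flash events to override.
; On BeginPlay it gets the audio manager from BP_RhythmGameMode and binds those events to its matching music cues.
; Play triggers Beat, with optional name printing for debugging.
; GetIsLevelActive returns true only when both the audio manager's level and the assigned LevelCrystal are active.
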(event Custom|Laser)

(event Custom|Beat
  (if (Variables|Default|GetPrintName)
    (Development|PrintString (Variables|Default|GetObjectName) true true "(R=0.000000,G=0.660000,B=1.000000,A=1.000000)" 0.4)))

(event Custom|Kick)

(event Custom|Marker
  (params (MarkerType :type String)))

(event Custom|Snare)

(event Custom|Flash)

(event EventBeginPlay
  (bind _asbp_rhythm_game_mode (Utilities|Casting|CastToBP_RhythmGameMode (Game|GetGameMode)))
  (bind _audiomanager (Default|GetAudioManager _asbp_rhythm_game_mode))
  (EventDispatchers|BindEventtoKickStarted _audiomanager (delegate Custom|Kick))
  (EventDispatchers|BindEventtoSnareStarted _audiomanager (delegate Custom|Snare))
  (EventDispatchers|BindEventtoLaserStarted _audiomanager (delegate Custom|Laser))
  (EventDispatchers|BindEventtoMarkerStarted _audiomanager (delegate Custom|Marker))
  (EventDispatchers|BindEventtoFlashStarted _audiomanager (delegate Custom|Flash)))

(fn ConstructionScript)

(fn Play
  (CallFunction|Beat)
  (if (Variables|Default|GetPrintName)
    (Development|PrintString (Variables|Default|GetObjectName) true true "(R=0.000000,G=0.660000,B=1.000000,A=1.000000)" 0.4)))

(fn GetIsLevelActive
  (bind _asbp_rhythm_game_mode (Utilities|Casting|CastToBP_RhythmGameMode (Game|GetGameMode)))
  (bind _audiomanager (Default|GetAudioManager _asbp_rhythm_game_mode))
  (bind _asbp_interactable_crystal (Utilities|Casting|CastToBP_Interactable_Crystal (Variables|Default|GetLevelCrystal)))
  (if (and (Variables|/Game/Blueprints/BP_AudioManager.BP_AudioManager_C|GetIsLevelActive _audiomanager) (Variables|/Game/Blueprints/BP_Interactable_Crystal.BP_Interactable_Crystal_C|GetIsActive _asbp_interactable_crystal))
    (LocalVariables|SetFinalBool true)
    (else
      (LocalVariables|SetFinalBool false)))
  (return (LocalVariables|GetFinalBool)))