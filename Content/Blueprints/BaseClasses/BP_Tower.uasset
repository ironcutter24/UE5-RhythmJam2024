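; BP_Tower is a beat-driven tower that detects when its expanding particle pulse reaches the player, currently only printing the result.
; Each EventBeat resets a beat timer and plays a timeline that bobs the top mesh.
; On async physics ticks, if the player is inside the volume with a clear horizontal trace, it estimates hits analytically, comparing 2D distance beyond the emitter radius against particle speed times beat time using a remainder test.
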(event EventBeginPlay
  (|CallParentFunction)
  ;[1 1 1] Init TopMeshStartLocation
  (Variables|Default|SetTopMeshStartLocation (.location (Transformation|GetRelativeTransform (Variables|Default|GetCylinder1)))))

(event EventEventBeat
  ;[1 1 1] Reset TimeFromBeat
  (Variables|Default|SetTimeFromBeat 0.0)
  ;[1 1 1] Animation
  (bind _pulseoffset (Timeline|Timeline PlayFromStart)
    (:Update
      (Transformation|SetRelativeLocation (Variables|Default|GetCylinder1) (+ (Math|Vector|MakeVector 0.0 0.0 _pulseoffset) (Variables|Default|GetTopMeshStartLocation)) false false))))

(event EventAsyncPhysicsTick
  (params (DeltaSeconds :type Float%20%28single-precision%29) (SimSeconds :type Float%20%28single-precision%29))
  (bind _returnvalue (Game|GetPlayerCharacter 0))
  (bind _returnvalue_2 (Transformation|GetActorTransform))
  (bind _returnvalue_3 (Transformation|GetActorTransform _returnvalue))
  (bind _returnvalue_4 (+ (.z (.location _returnvalue_2)) 1e+02))
  ;[1 1 1] Add to TimeFromBeat
  (Variables|Default|SetTimeFromBeat (+ DeltaSeconds (Variables|Default|GetTimeFromBeat)))
  ;[1 1 1] Is Player in Volume
  (if (Collision|IsOverlappingActor (Variables|Default|GetVolume) _returnvalue :!class /Script/Engine.PrimitiveComponent)
    ;[1 1 1] Has line of sight
    (bind _returnvalue_5 (Collision|LineTraceByChannel (Math|Vector|MakeVector (.x (.location _returnvalue_2)) (.y (.location _returnvalue_2)) _returnvalue_4) (Math|Vector|MakeVector (.x (.location _returnvalue_3)) (.y (.location _returnvalue_3)) _returnvalue_4) "TraceTypeQuery1" false 0 "ForOneFrame"))
    (if (not _returnvalue_5)
      (if (or (< (.Remainder (Math|Float|Division(WholeandRemainder) (- (Math|Vector|Distance2D(Vector) (Math|Conversions|ToVector2D(Vector) (.location (Transformation|GetActorTransform))) (Math|Conversions|ToVector2D(Vector) (.location (Transformation|GetActorTransform (Game|GetPlayerCharacter 0))))) (Variables|Default|GetEmitterRadius)) (* (Variables|Default|GetParticleSpeed) (Variables|Default|GetTimeFromBeat)))) 0.5) (> (.Remainder (Math|Float|Division(WholeandRemainder) (- (Math|Vector|Distance2D(Vector) (Math|Conversions|ToVector2D(Vector) (.location (Transformation|GetActorTransform))) (Math|Conversions|ToVector2D(Vector) (.location (Transformation|GetActorTransform (Game|GetPlayerCharacter 0))))) (Variables|Default|GetEmitterRadius)) (* (Variables|Default|GetParticleSpeed) (Variables|Default|GetTimeFromBeat)))) (- (* (Variables|Default|GetParticleSpeed) (Variables|Default|GetTimeFromBeat)) 0.5)))
        (Development|PrintString "Player hit: True" false)
        (else
          (Development|PrintString "Player hit: False" false))))))

(fn ConstructionScript
  (|CallParentFunction))

(fn Play
  (|CallParentFunction))