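; Checkpoint actor that saves the player's location to the custom game instance and lights three crystal torch child actors when activated.
; The first player overlap with its trigger sphere calls SetCheckpoint, then lights the torches sequentially through a delayed loop before marking itself lit.
; BeginPlay has an instant-light path meant for the current checkpoint, but its check compares the game instance itself to this actor.
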(event OnComponentBeginOverlap(TriggerSphere)
  (params (OverlappedComponent :type Primitive%20Component%20Object%20Reference) (OtherActor :type Actor%20Object%20Reference) (OtherComp :type Primitive%20Component%20Object%20Reference) (OtherBodyIndex :type Integer) (bFromSweep :type Boolean) (SweepResult :type Hit%20Result%20Structure%20%28by%20ref%29))
  (if (not (Variables|Default|GetIsLit))
    ;[1 1 1] Set as current checkpoint
    (if (== OtherActor (Game|GetPlayerCharacter 0))
      (bind _ascustom_game_instance (Utilities|Casting|CastToCustomGameInstance (Game|GetGameInstance)))
      (Default|SetCheckpoint _ascustom_game_instance (Transformation|GetActorLocation (Game|GetPlayerCharacter 0)))
      ;[1 1 1] Gradually light torches
      (bind _array_element (Utilities|ForEachLoopDelay (Variables|Default|GetChildActors) (Variables|Default|GetLightDelay))
        (:LoopBody
          (CallFunction|LightChildTorch _array_element))
        (:Completed
          (Variables|Default|SetIsLit true))))))

(event EventBeginPlay
  ;[1 1 1] Init ChildActors array
  (Variables|Default|SetChildActors (Utilities|Array|MakeArray (Variables|Default|GetBP_CPCrystals) (Variables|Default|GetBP_CPCrystals1) (Variables|Default|GetBP_CPCrystals2)))
  ;[1 1 1] Check if this is current checkpoint
  (bind _ascustom_game_instance (Utilities|Casting|CastToCustomGameInstance (Game|GetGameInstance)))
  (if (== _ascustom_game_instance self)
    ;[1 1 1] Instantly light torches
    (for _array_element (Variables|Default|GetChildActors)
      (CallFunction|LightChildTorch _array_element))
    (Variables|Default|SetIsLit true)))

(fn ConstructionScript)

(fn LightChildTorch
  (params (Child%20Actor :type Child%20Actor%20Component%20Object%20Reference))
  (bind _asbp_cpcrystals (Utilities|Casting|CastToBP_CPCrystals (Variables|/Script/Engine.ChildActorComponent|GetChildActor Child%20Actor))
    (:then
      (Default|LightTorch _asbp_cpcrystals))
    (:CastFailed
      (Development|PrintString "BP_CPCrystals cast failed" true true "(R=1.000000,G=0.000000,B=0.018907,A=1.000000)"))))