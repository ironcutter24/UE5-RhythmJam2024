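; Music manager that plays the FMOD soundtrack and turns its timeline into rhythm events for gameplay.
; Beat callbacks broadcast kick, snare and laser events on set beats of a 6/8 pattern, and markers are re-broadcast by name.
; ProcessMusicObjects, not called here, maps nearest tower and laser distances to FMOD parameters, though the laser's parameter is unnamed and piano distance goes unused.
; A dash timing-window chain is disconnected.
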(event Custom|On%20Tempo
  (params (Bar :type Integer) (Beat :type Integer) (Position :type Integer) (Tempo :type Float%20%28single-precision%29) (TimeSignatureUpper :type Integer) (TimeSignatureLower :type Integer))
  (Utilities|FlowControl|Sequence
    (:then_0
      ;[1 1 1] Init tempo variables
      (bind _baroveramount (CallFunction|GetBarOverAmount Bar 2))
      (Variables|Default|SetBarOverTwo _baroveramount))
    (:then_1
      (Variables|Default|SetBeat Beat))
    (:then_2
      (Utilities|FlowControl|Sequence
        (:then_0
          ;[1 1 1] Kick
          (if (== 1 (Variables|Default|GetBeat))
            (Default|CallKickStarted)))
        (:then_1
          ;[1 1 1] Snare
          (if (and (== 1 (Variables|Default|GetBarOverTwo)) (== 5 (Variables|Default|GetBeat)))
            (Default|CallSnareStarted)))
        (:then_2
          ;[1 1 1] Laser
          (if (== 3 (Variables|Default|GetBeat))
            (Default|CallLaserStarted)))))
    (:then_3)))

(event Custom|On%20Marker
  (params (Name :type String) (Position :type Integer))
  (Default|CallMarkerStarted Name))

(event EventBeginPlay
  (Utilities|FlowControl|Sequence
    (:then_0
      ;[1 1 1] Init FMOD
      (bind _returnvalue (AddComponent|AddFMODAudioComponent false))
      (bind _output_get (Variables|Default|SetFMOD%20Component _returnvalue))
      (Class|FMODAudioComponent|SetEvent _output_get "/Game/FMOD/Events/OST.OST")
      (EventDispatchers|BindEventtoOnTimelineBeat _output_get (delegate Custom|On%20Tempo))
      (EventDispatchers|BindEventtoOnTimelineMarker _output_get (delegate Custom|On%20Marker))
      (Variables|/Script/FMODStudio.FMODAudioComponent|SetbEnableTimelineCallbacks _output_get true)
      (Class|FMODAudioComponent|Play _output_get))
    (:then_1
      ;[1 1 1] Set FMOD parameters
      (Class|FMODAudioComponent|SetParameter (Variables|Default|GetFMOD%20Component) "Kick" 1.0)
      (Class|FMODAudioComponent|SetParameter (Variables|Default|GetFMOD%20Component) "Snare" 1.0)
      (Class|FMODAudioComponent|SetParameter (Variables|Default|GetFMOD%20Component) "Piano_Harmonics" 1.0))))

(fn ConstructionScript)

(fn TriggerAction
  (params (Actors :type Array%20of%20Actor%20Object%20References))
  (for _array_element Actors
    (bind _asbp_music_object (Utilities|Casting|CastToBP_MusicObject _array_element))
    (Default|Play _asbp_music_object)))

(fn GetBarOverAmount
  (params (Bar :type Integer) (Amount :type Integer))
  (return (+ (.Remainder (Math|Float|Division(WholeandRemainder) (- Bar 1) (Math|Conversions|ToFloat(Integer) Amount))) 1)))

(fn GetBeatDuration
  (return (/ 6e+01 (Variables|Default|GetBPM))))

(fn GetBarDuration
  (bind _seconds (CallFunction|GetBeatDuration))
  (return (* _seconds (LocalVariables|GetBeatsInBar))))

(fn ProcessMusicObjects
  (params (MusicObjects :type Array%20of%20Actor%20Object%20References))
  (for _array_element MusicObjects :!label _label
    (if (== (Utilities|GetClass _array_element) "/Game/Blueprints/BP_KickTower.BP_KickTower_C")
      (if (< (Class|KismetMathLibrary|VectorDistance2DSquared (.location (Transformation|GetActorTransform _array_element)) (Transformation|GetActorLocation (Game|GetPlayerController 0))) (LocalVariables|GetKickSqrDist))
        (LocalVariables|SetKickSqrDist (Class|KismetMathLibrary|VectorDistance2DSquared (.location (Transformation|GetActorTransform _array_element)) (Transformation|GetActorLocation (Game|GetPlayerController 0))))
        (if true :!label _label_2
          (goto _label Next%20Body)))
      (elif (== (Utilities|GetClass _array_element) "/Game/Blueprints/BP_SnareTower.BP_SnareTower_C")
        (if (< (Class|KismetMathLibrary|VectorDistance2DSquared (.location (Transformation|GetActorTransform _array_element)) (Transformation|GetActorLocation (Game|GetPlayerController 0))) (LocalVariables|GetSnareSqrDist))
          (LocalVariables|SetSnareSqrDist (Class|KismetMathLibrary|VectorDistance2DSquared (.location (Transformation|GetActorTransform _array_element)) (Transformation|GetActorLocation (Game|GetPlayerController 0))))
          (goto _label_2))
        (elif (== (Utilities|GetClass _array_element) "/Game/Blueprints/BP_Laser.BP_Laser_C")
          (if (< (Class|KismetMathLibrary|VectorDistance2DSquared (.location (Transformation|GetActorTransform _array_element)) (Transformation|GetActorLocation (Game|GetPlayerController 0))) (LocalVariables|GetLaserSqrDist))
            (LocalVariables|SetLaserSqrDist (Class|KismetMathLibrary|VectorDistance2DSquared (.location (Transformation|GetActorTransform _array_element)) (Transformation|GetActorLocation (Game|GetPlayerController 0))))
            (goto _label_2))
          (elif (== (Utilities|GetClass _array_element) "/Game/Giacomo_Test/PianoRoll/BP_PianoRollManager.BP_PianoRollManager_C")
            (if (< (Class|KismetMathLibrary|VectorDistance2DSquared (.location (Transformation|GetActorTransform _array_element)) (Transformation|GetActorLocation (Game|GetPlayerController 0))) (LocalVariables|GetPianoSqrDist))
              (LocalVariables|SetPianoSqrDist (Class|KismetMathLibrary|VectorDistance2DSquared (.location (Transformation|GetActorTransform _array_element)) (Transformation|GetActorLocation (Game|GetPlayerController 0))))
              (goto _label_2)))))))
  (bind _value (CallFunction|NormalizeSqrDistance (LocalVariables|GetKickSqrDist)))
  (Class|FMODAudioComponent|SetParameter (Variables|Default|GetFMOD%20Component) "Kick" _value)
  (bind _value_2 (CallFunction|NormalizeSqrDistance (LocalVariables|GetSnareSqrDist)))
  (Class|FMODAudioComponent|SetParameter (Variables|Default|GetFMOD%20Component) "Snare" _value_2)
  (bind _value_3 (CallFunction|NormalizeSqrDistance (LocalVariables|GetLaserSqrDist)))
  (Class|FMODAudioComponent|SetParameter (Variables|Default|GetFMOD%20Component) "Laser" _value_3))

(fn NormalizeSqrDistance
  (params (SqrDist :type Float%20%28double-precision%29))
  (return (- 1.0 (Math|Float|Clamp(Float) (/ (Math|Float|Sqrt SqrDist) 1e+03)))))