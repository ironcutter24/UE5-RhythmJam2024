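; BP_WallUpToDown is a wall actor that slides vertically down from its starting position when LevelStart fires.
; BeginPlay caches the Wall component's relative location, and LevelStart plays a Timeline that offsets it along Z by the track value times WallHeight.
; The IsRise function sets the direction by mapping its boolean to a plus or minus sign, and returns false here, so the wall descends.
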(event Custom|Level%20Start
  (bind _value (CallFunction|IsRise))
  (bind _newtrack_0 (Timeline|Timeline PlayFromStart)
    (:Update
      (Transformation|SetRelativeLocation (Variables|Default|GetWall) (+ (Math|Vector|MakeVector 0.0 0.0 (* _newtrack_0 (- (* (Math|Conversions|ToInteger(Boolean) _value) 2) 1) (Variables|Default|GetWallHeight))) (Variables|Default|GetStartPosition)) false false))))

(event EventBeginPlay
  (Variables|Default|SetStartPosition (.location (Transformation|GetRelativeTransform (Variables|Default|GetWall)))))

(fn ConstructionScript)

(fn IsRise
  (return false))