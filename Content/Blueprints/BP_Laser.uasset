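; A laser turret that sweeps a Niagara beam back and forth in response to beat events.
; Each beat alternates the LaserTurn timeline between forward and reverse, yawing the emitter by a configurable angle and starting direction.
; On timeline updates, a visibility line trace along the emitter's right vector sets the beam end at the hit point or maximum ray length, with no damage logic.
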(event EventBeginPlay
  (|CallParentFunction)
  (bind _returnvalue (AddComponent|AddNiagaraComponent false (Transformation|GetRelativeTransform (Variables|Default|GetLaserEmitter))))
  (bind _output_get (Variables|Default|SetLaserParticle _returnvalue))
  (CallFunction|SetBeamEnd _output_get "0, 0, 0"))

(event Collision|EventActorBeginOverlap
  (params (OtherActor :type Actor%20Object%20Reference))
  (|CallParentFunction OtherActor) ; This node is disabled and will not be called.\nDrag off pins to build functionality.
)

(event EventEventBeat
  (bind _laserparticle (Variables|Default|GetLaserParticle))
  (bind _raylenght (Variables|Default|GetRayLenght))
  (bind _laseremitter (Variables|Default|GetLaserEmitter))
  (bind _laseremitter_2 (Variables|Default|GetLaserEmitter))
  (bind _returnvalue (Transformation|GetWorldLocation _laseremitter_2))
  (bind _returnvalue_2 (Math|Vector|GetRightVector _laseremitter))
  (bind _returnvalue_3 (* _returnvalue_2 _raylenght))
  (bind _returnvalue_4 (+ _returnvalue _returnvalue_3))
  (Utilities|FlowControl|FlipFlop
    (:A
      (bind _zrotation (Timeline|LaserTurn PlayFromStart)
        (:Update
          ;[1 1 1] Rotate turret
          (Transformation|SetRelativeRotation (Variables|Default|GetLaserEmitter) (Math|Rotator|MakeRotator 0.0 0.0 (* _zrotation (- (* (Math|Conversions|ToInteger(Boolean) (Variables|Default|GetStartClockwise)) 2) 1) (Variables|Default|GetTurnAngle))) false false)
          (bind (_outhit _returnvalue_5) (Collision|LineTraceByChannel _returnvalue _returnvalue_4 "TraceTypeQuery1" false 0 "ForOneFrame"))
          ;[1 1 1] Set Laser beam end
          (if _returnvalue_5
            (CallFunction|SetBeamEnd _laserparticle (.location _outhit))
            (else
              (CallFunction|SetBeamEnd _laserparticle _returnvalue_4))))))
    (:B
      (Timeline|LaserTurn ReverseFromEnd))))

(fn ConstructionScript
  (|CallParentFunction))

(fn SetBeamEnd
  (params (Particle :type Niagara%20Component%20Object%20Reference) (Location :type Vector))
  (Class|NiagaraComponent|SetNiagaraVariableVec3 Particle "Beam End" Location))