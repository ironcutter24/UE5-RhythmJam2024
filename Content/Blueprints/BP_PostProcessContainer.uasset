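; BP_PostProcessContainer is a volume Blueprint that switches off the player's rain effect while the player is inside its Collider.
; On begin and end overlap with an actor tagged "Player", it fetches the rain component from player character 0 through the IGetRain interface message.
; Entering deactivates that component, and leaving reactivates it with a reset.
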(event OnComponentBeginOverlap(Collider)
  (params (OverlappedComponent :type Primitive%20Component%20Object%20Reference) (OtherActor :type Actor%20Object%20Reference) (OtherComp :type Primitive%20Component%20Object%20Reference) (OtherBodyIndex :type Integer) (bFromSweep :type Boolean) (SweepResult :type Hit%20Result%20Structure%20%28by%20ref%29))
  (if (Actor|ActorHasTag OtherActor "Player")
    (bind _raincomponent (Class|IPlayerUtilities|IGetRain(Message) (Game|GetPlayerCharacter 0)))
    (Components|Activation|Deactivate _raincomponent)))

(event OnComponentEndOverlap(Collider)
  (params (OverlappedComponent :type Primitive%20Component%20Object%20Reference) (OtherActor :type Actor%20Object%20Reference) (OtherComp :type Primitive%20Component%20Object%20Reference) (OtherBodyIndex :type Integer))
  (if (Actor|ActorHasTag OtherActor "Player")
    (bind _raincomponent (Class|IPlayerUtilities|IGetRain(Message) (Game|GetPlayerCharacter 0)))
    (Components|Activation|Activate _raincomponent true)))

(fn ConstructionScript)