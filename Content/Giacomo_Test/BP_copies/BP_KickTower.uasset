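; BP_KickTower is a tower Blueprint, in a test copies folder, that fires a "kick" through its Play function.
; Play creates a level sequence player for the IntensityChange sequence, starts it, then calls the kick dispatcher and prints a debug string.
; The event graph holds only disabled default stubs, so nothing in this file triggers Play itself.
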(event EventBeginPlay
  (|CallParentFunction) ; This node is disabled and will not be called.\nDrag off pins to build functionality.
)

(event Collision|EventActorBeginOverlap
  (params (OtherActor :type Actor%20Object%20Reference))
  (|CallParentFunction OtherActor) ; This node is disabled and will not be called.\nDrag off pins to build functionality.
)

(event EventTick
  (params (DeltaSeconds :type Float%20%28single-precision%29))
  (|CallParentFunction DeltaSeconds) ; This node is disabled and will not be called.\nDrag off pins to build functionality.
)

(fn ConstructionScript
  (|CallParentFunction))

(fn Play
  (bind _outactor (Sequencer|Player|CreateLevelSequencePlayer "/Game/Giacomo_Test/IntensityChange.IntensityChange"))
  (Sequencer|Player|Play (Variables|/Script/LevelSequence.LevelSequenceActor|GetSequencePlayer _outactor) :!class /Script/MovieScene.MovieSceneSequencePlayer)
  (Default|CallKickDispatcher)
  (Development|PrintString "Hello"))