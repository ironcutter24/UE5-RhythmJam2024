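; BP_AudioManager plays the FMOD OST event and triggers hazard towers in time with the music.
; Timeline beat callbacks use bar and beat modulo checks to pick kick or snare beats, then find all BP_KickTower or BP_SnareTower actors.
; TriggerAction casts those actors to BP_BaseHazard and calls Play.
; Timeline markers are printed, and the Piano case is an unfinished stub.
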(event Custom|On%20Tempo
  (params (Bar :type Integer) (Beat :type Integer) (Position :type Integer) (Tempo :type Float%20%28single-precision%29) (TimeSignatureUpper :type Integer) (TimeSignatureLower :type Integer))
  (bind _returnvalue (Math|Conversions|ToFloat(Integer) Beat))
  (bind _returnvalue_2 (- _returnvalue 1.0))
  (bind _remainder (Math|Float|Division(WholeandRemainder) _returnvalue_2 3.0))
  (Utilities|FlowControl|Sequence
    (:then_0
      ;[1 1 1] Kick
      (if (== _remainder 0.0)
        (bind _outactors (Actor|GetAllActorsOfClass "/Game/Giacomo_Test/BP_copies/BP_KickTower.BP_KickTower_C"))
        (CallFunction|TriggerAction _outactors)))
    (:then_1
      ;[1 1 1] Snare
      (if (and (== (.Remainder (Math|Float|Division(WholeandRemainder) (- (Math|Conversions|ToFloat(Integer) Bar) 1.0) 2.0)) 0.0) (== _remainder 2.0))
        (bind _outactors_2 (Actor|GetAllActorsOfClass "/Game/Giacomo_Test/BP_copies/BP_SnareTower.BP_SnareTower_C"))
        (CallFunction|TriggerAction _outactors_2)))))

(event Custom|On%20Marker
  (params (Name :type String) (Position :type Integer))
  (Development|PrintString Name)
  (switch string Name
    (:Piano
      (Actor|GetAllActorsOfClass 0))))

(event EventBeginPlay
  (bind _returnvalue (AddComponent|AddFMODAudioComponent false))
  (Class|FMODAudioComponent|SetEvent _returnvalue "/Game/FMOD/Events/OST.OST")
  (EventDispatchers|BindEventtoOnTimelineBeat _returnvalue (delegate Custom|On%20Tempo))
  (EventDispatchers|BindEventtoOnTimelineMarker _returnvalue (delegate Custom|On%20Marker))
  (Variables|/Script/FMODStudio.FMODAudioComponent|SetbEnableTimelineCallbacks _returnvalue true)
  (Class|FMODAudioComponent|Play _returnvalue))

(fn ConstructionScript)

(fn TriggerAction
  (params (Actors :type Array%20of%20Actor%20Object%20References))
  (for _array_element Actors
    (bind _asbp_base_hazard (Utilities|Casting|CastToBP_BaseHazard _array_element))
    (Default|Play _asbp_base_hazard)))