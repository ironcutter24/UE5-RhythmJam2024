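; BP_PianoNote is a piano roll note actor that travels along the world X axis and bursts when it hits something.
; Tick offsets its location by NoteSpeed scaled by delta time, without sweeping.
; The first BoxCollision overlap with any actor prints that actor's name, destroys the box and note components, activates PianoRoll2DExplosion, and sets a short lifespan so the actor removes itself afterwards.
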(event OnComponentBeginOverlap(BoxCollision)
  (params (OverlappedComponent :type Primitive%20Component%20Object%20Reference) (OtherActor :type Actor%20Object%20Reference) (OtherComp :type Primitive%20Component%20Object%20Reference) (OtherBodyIndex :type Integer) (bFromSweep :type Boolean) (SweepResult :type Hit%20Result%20Structure%20%28by%20ref%29))
  (Development|PrintString (Utilities|GetObjectName OtherActor))
  (Components|DestroyComponent (Variables|Default|GetBoxCollision))
  (Components|DestroyComponent (Variables|Default|GetPianoNote))
  (Components|Activation|Activate (Variables|Default|GetPianoRoll_2D_Explosion) false)
  (Actor|SetLifeSpan 2.0))

(event Collision|EventActorBeginOverlap
  (params (OtherActor :type Actor%20Object%20Reference)))

(event EventTick
  (params (DeltaSeconds :type Float%20%28single-precision%29))
  (Transformation|SetActorLocation (+ (Math|Vector|MakeVector (* DeltaSeconds (Variables|Default|GetNoteSpeed)) 0.0 0.0) (Transformation|GetActorLocation)) false false))

(fn ConstructionScript)