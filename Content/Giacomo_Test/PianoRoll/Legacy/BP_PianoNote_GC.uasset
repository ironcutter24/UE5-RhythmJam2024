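; Legacy piano roll note actor that slides along world X and switches its Geometry Collection to physics simulation when hit.
; BeginPlay turns simulation off, and Tick moves the actor by NoteSpeed scaled by delta time, without sweeping.
; A hit on BoxCollision turns simulation on and prints the other actor's name for debugging.
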(event OnComponentHit(BoxCollision)
  (params (HitComponent :type Primitive%20Component%20Object%20Reference) (OtherActor :type Actor%20Object%20Reference) (OtherComp :type Primitive%20Component%20Object%20Reference) (NormalImpulse :type Vector :default "0, 0, 0") (Hit :type Hit%20Result%20Structure%20%28by%20ref%29))
  (Physics|SetSimulatePhysics (Variables|Default|GetPianoNote_GeomCollec) true)
  (Development|PrintString (Utilities|GetObjectName OtherActor)))

(event EventBeginPlay
  (Physics|SetSimulatePhysics (Variables|Default|GetPianoNote_GeomCollec) false))

(event Collision|EventActorBeginOverlap
  (params (OtherActor :type Actor%20Object%20Reference)))

(event EventTick
  (params (DeltaSeconds :type Float%20%28single-precision%29))
  (Transformation|SetActorLocation (+ (Math|Vector|MakeVector (* DeltaSeconds (Variables|Default|GetNoteSpeed)) 0.0 0.0) (Transformation|GetActorLocation)) false false))

(fn ConstructionScript)