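; Piano roll manager for the rhythm game that spawns visual notes from six child-actor emitters for one instrument source: piano chord, piano melody or cello melody.
; On BeginPlay it colors each emitter with that source's materials from BP_RhythmGameMode.
; While the level is active, Marker events are filtered by source and mapped by name to chord shapes or single-lane patterns, which PlayChord sends to the matching emitters to spawn notes.
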(event EventBeginPlay
  ;[1 1 1] MakeArray
  (|CallParentFunction)
  (bind _output_get (Variables|Default|SetEmitters (Utilities|Array|MakeArray (Variables|Default|GetBP_PianoRollEmitter1) (Variables|Default|GetBP_PianoRollEmitter2) (Variables|Default|GetBP_PianoRollEmitter3) (Variables|Default|GetBP_PianoRollEmitter4) (Variables|Default|GetBP_PianoRollEmitter5) (Variables|Default|GetBP_PianoRollEmitter%206))))
  ;[1 1 1] Update Colors from PianoRollColorsManager
  (bind _asbp_rhythm_game_mode (Utilities|Casting|CastToBP_RhythmGameMode (Game|GetGameMode)))
  (switch Utilities|FlowControl|Switch|SwitchonMarkerType (Variables|Default|GetPianoRollSource)
    (:NewEnumerator0
      (Variables|Default|SetCurrentMaterials (Variables|/Game/Blueprints/BP_RhythmGameMode.BP_RhythmGameMode_C|GetPianoChordMats _asbp_rhythm_game_mode)))
    (:NewEnumerator1
      (Variables|Default|SetCurrentMaterials (Variables|/Game/Blueprints/BP_RhythmGameMode.BP_RhythmGameMode_C|GetPianoMelodyMats _asbp_rhythm_game_mode)))
    (:NewEnumerator2
      (Variables|Default|SetCurrentMaterials (Variables|/Game/Blueprints/BP_RhythmGameMode.BP_RhythmGameMode_C|GetCelloMelodyMats _asbp_rhythm_game_mode))))
  (for (_array_element _array_index) _output_get
    (bind _asbp_piano_roll_emitter (Utilities|Casting|CastToBP_PianoRollEmitter (Variables|/Script/Engine.ChildActorComponent|GetChildActor _array_element)))
    (Default|SetNoteEmitterColorEvent _asbp_piano_roll_emitter (Utilities|Array|Get(acopy) (Variables|Default|GetCurrentMaterials) _array_index))))

(event EventMarker
  (params (MarkerType :type String))
  (bind _chordshapes (Variables|Default|GetChordShapes))
  (if (CallFunction|GetIsLevelActive)
    (switch Utilities|FlowControl|Switch|SwitchonMarkerType (Variables|Default|GetPianoRollSource)
      (:NewEnumerator0
        ;[1 1 1] PianoChords
        (if (Utilities|String|Contains MarkerType "C")
          (switch string MarkerType
            (:L1_C1
              (Variables|Default|SetCurrent%20Chord%20Shape_0 (.notes (Utilities|Array|Get(acopy) _chordshapes))))
            (:L1_C2
              (Variables|Default|SetCurrent%20Chord%20Shape_0 (.notes (Utilities|Array|Get(acopy) _chordshapes 1))))
            (:L1_C3
              (Variables|Default|SetCurrent%20Chord%20Shape_0 (.notes (Utilities|Array|Get(acopy) _chordshapes 2))))
            (:L1_C4
              (Variables|Default|SetCurrent%20Chord%20Shape_0 (.notes (Utilities|Array|Get(acopy) _chordshapes 2)))))
          (CallFunction|PlayChord (Variables|Default|GetCurrent%20Chord%20Shape_0) :!label _label)))
      (:NewEnumerator1
        ;[1 1 1] PianoMelody
        (if (Utilities|String|Contains MarkerType "M")
          (switch string MarkerType
            (:L1_M1
              (Variables|Default|SetCurrent%20Chord%20Shape_0 (Utilities|Array|MakeArray true false false false false false))
              (goto _label))
            (:L1_M2
              (Variables|Default|SetCurrent%20Chord%20Shape_0 (Utilities|Array|MakeArray false true false false false false))
              (goto _label))
            (:L1_M3
              (Variables|Default|SetCurrent%20Chord%20Shape_0 (Utilities|Array|MakeArray false false true false false false))
              (goto _label))
            (:L1_M4
              (Variables|Default|SetCurrent%20Chord%20Shape_0 (Utilities|Array|MakeArray false false false true false false))
              (goto _label))
            (:L1_M5
              (Variables|Default|SetCurrent%20Chord%20Shape_0 (Utilities|Array|MakeArray false false false false true false))
              (goto _label))
            (:L1_M6
              (Variables|Default|SetCurrent%20Chord%20Shape_0 (Utilities|Array|MakeArray false false false false false true))
              (goto _label)))))
      (:NewEnumerator2
        ;[1 1 1] CelloMelody
        (if (Utilities|String|Contains MarkerType "H")
          (switch string MarkerType
            (:L1_H1
              (Variables|Default|SetCurrent%20Chord%20Shape_0 (Utilities|Array|MakeArray true false false false false false))
              (goto _label))
            (:L1_H2
              (Variables|Default|SetCurrent%20Chord%20Shape_0 (Utilities|Array|MakeArray false true false false false false))
              (goto _label))
            (:L1_H3
              (Variables|Default|SetCurrent%20Chord%20Shape_0 (Utilities|Array|MakeArray false false true false false false))
              (goto _label))
            (:L1_H4
              (Variables|Default|SetCurrent%20Chord%20Shape_0 (Utilities|Array|MakeArray false false false true false false))
              (goto _label))
            (:L1_H5
              (Variables|Default|SetCurrent%20Chord%20Shape_0 (Utilities|Array|MakeArray false false false false true false))
              (goto _label))
            (:L1_H6
              (Variables|Default|SetCurrent%20Chord%20Shape_0 (Utilities|Array|MakeArray false false false false false true))
              (goto _label))))))))

(fn ConstructionScript)

(fn PlayChord
  (params (CurrentChordShape :type Array%20of%20Booleans))
  (for (_array_element _array_index) CurrentChordShape
    (if _array_element
      (bind _asbp_piano_roll_emitter (Utilities|Casting|CastToBP_PianoRollEmitter (Variables|/Script/Engine.ChildActorComponent|GetChildActor (Utilities|Array|Get(acopy) (Variables|Default|GetEmitters) _array_index))))
      (Default|SpawnNote _asbp_piano_roll_emitter (Variables|Default|GetNotesSpeed) (Variables|Default|GetNotesLifetime)))))

(fn ParseMarker
  (params (MarkerName :type String) (MarkerType :type MarkerType%20Enum :default "MarkerType_MAX"))
  (switch Utilities|FlowControl|Switch|SwitchonMarkerType MarkerType
    (:NewEnumerator0
      (if (Utilities|String|Contains MarkerName "C")
        (Development|PrintString MarkerName true true "(R=0.000000,G=0.250000,B=1.000000,A=1.000000)")
        (switch string MarkerName
          (:L1_C1
            (bind _output_get (LocalVariables|SetCurrentShape (Utilities|Array|Get(acopy) (Variables|Default|GetChordShapes))))
            (return (Utilities|Struct|BreakChordShape _output_get))))))))