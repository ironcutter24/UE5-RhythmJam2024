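; BP_KickLight is a light actor that pulses its point light whenever the kick tower signals a kick.
; On BeginPlay it finds the first BP_KickTower in the level and binds its light event to that tower's kick dispatcher.
; Each kick sets the light color and restarts a timeline whose curve, scaled by a maximum intensity, drives the light's brightness.
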(event Custom|LightIntensityEvent
  (bind _pointlight (Variables|Default|GetPointLight))
  (Rendering|Components|Light|SetLightColor _pointlight (Math|Conversions|ToLinearColor(Color) (Variables|Default|GetLightColor)) true)
  (bind _lightintensityanim (Timeline|LightAnimation PlayFromStart)
    (:Update
      (Rendering|Components|Light|SetIntensity _pointlight (* _lightintensityanim (Variables|Default|GetMaxLightInt))))))

(event EventBeginPlay
  (bind _outactors (Actor|GetAllActorsOfClass "/Game/Giacomo_Test/BP_copies/BP_KickTower.BP_KickTower_C"))
  (bind _asbp_kick_tower (Utilities|Casting|CastToBP_KickTower (Utilities|Array|Get(acopy) _outactors)))
  (EventDispatchers|BindEventtoKickDispatcher _asbp_kick_tower (delegate Custom|LightIntensityEvent)))

(event Collision|EventActorBeginOverlap
  (params (OtherActor :type Actor%20Object%20Reference)))

(event EventTick
  (params (DeltaSeconds :type Float%20%28single-precision%29)))

(fn ConstructionScript)